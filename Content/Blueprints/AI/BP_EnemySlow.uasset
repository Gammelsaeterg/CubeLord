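; BP_EnemySlow is a slow enemy character with a spear that randomizes its walk speed on spawn.
; Attacks play a quick montage and set an attacking flag, with separate events toggling spear collision.
; A spear overlap with the player only prints its name and disables collision, with no damage applied.
; When hit, it detaches from its controller, ragdolls body and spear, then destroys itself after a delay.
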(event OnComponentBeginOverlap(Spear)
  (params (OverlappedComponent :type Primitive%20Component%20Object%20Reference) (OtherActor :type Actor%20Object%20Reference) (OtherComp :type Primitive%20Component%20Object%20Reference) (OtherBodyIndex :type Integer) (bFromSweep :type Boolean) (SweepResult :type Hit%20Result%20Structure%20%28by%20ref%29))
  (bind _asbp_player_character (Utilities|Casting|CastToBP_PlayerCharacter OtherActor))
  (Development|PrintString (Utilities|GetObjectName _asbp_player_character))
  (CallFunction|DisableWeaponCollision))

(event Custom|DisableWeaponCollision
  (Collision|SetCollisionEnabled (Variables|Default|GetSpear) "NoCollision"))

(event Custom|EnableWeaponCollision
  (Collision|SetCollisionEnabled (Variables|Default|GetSpear) "QueryAndPhysics"))

(event Custom|StartAttackSeqence
  (Animation|PlayAnimMontage "/Game/Meshes/Character/Animations/SlowEnemyAttackQuick_Montage.SlowEnemyAttackQuick_Montage" 1.0 "None")
  (Variables|Default|SetbIsAttacking true))

(event Custom|ActionAnimEnd
  (Variables|Default|SetbIsAttacking false))

(event Custom|ActionAnimStart
  (Variables|Default|SetbIsAttacking true))

(event Custom|AttackReceived
  (CallFunction|DestroySequence))

(event Custom|DestroySequence
  (Class|Pawn|DetachfromControllerPendingDestroy)
  (Collision|SetCollisionProfileName (Variables|Character|GetMesh) "Ragdoll" true :!class /Script/Engine.PrimitiveComponent)
  (Physics|SetSimulatePhysics (Variables|Character|GetMesh) true)
  (Collision|SetCollisionEnabled (Variables|Collision|GetCapsuleComponent) "NoCollision")
  (Utilities|FlowControl|Delay 1e+01)
  (Actor|DestroyActor))

(event EventBeginPlay
  (bind _charactermovement (Variables|Character|GetCharacterMovement))
  (Variables|/Script/Engine.CharacterMovementComponent|SetMaxWalkSpeed _charactermovement (+ (Variables|/Script/Engine.CharacterMovementComponent|GetMaxWalkSpeed _charactermovement) (Math|Random|RandomFloatinRange (* (Variables|Default|GetRandomWalkSpeedDeviation) -1.0) (Variables|Default|GetRandomWalkSpeedDeviation))))
  (Components|SkinnedMesh|SetPhysicsAsset (Variables|Character|GetMesh) "/Game/Meshes/Character/Mesh/SK_MannequinSlowEnemy_PhysicsAsset.SK_MannequinSlowEnemy_PhysicsAsset" false))

(fn ConstructionScript)