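; Cube pawn that, when hit, launches away from the hit location along the nearest X or Y axis.
; HitReceived snaps the direction with FindNearestDirection, then the LaunchCube timeline curve feeds swept FloatingPawnMovement.
; The same timeline drives trail particle speed, spawn rate and the glow intensity of a dynamic material.
; ShowBeam aims a beam particle at a given location, using DoOnce gates to toggle it with movement.
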(event Custom|HitReceived
  (params (HitFromLocation :type Vector))
  (bind _returnvalue (Transformation|GetActorLocation))
  (bind _returnvalue_2 (- (Math|Vector|MakeVector (.x HitFromLocation) (.y HitFromLocation) 0.0) (Math|Vector|MakeVector (.x _returnvalue) (.y _returnvalue) 0.0)))
  (bind _returnvalue_3 (Math|Vector|Normalize _returnvalue_2))
  ;[0.3782 0.2648 1] FindClosestXYDirection
  (bind (_outx _outy) (CallFunction|FindNearestDirection (.x _returnvalue_3) (.y _returnvalue_3)))
  (Variables|Default|SetCurrentLaunchDirection (* (Math|Vector|MakeVector (Math|Conversions|ToFloat(Integer) _outx) (Math|Conversions|ToFloat(Integer) _outy) 0.0) -1.0))
  ;[1 0 0.06404] CubeLaunch
  (bind (_direction _launchcurve _emitterspawnrate) (Timeline|LaunchCube PlayFromStart)
    (:Update
      (CallFunction|ControlEmitter _launchcurve _emitterspawnrate)
      (Class|PawnMovementComponent|AddInputVector (Variables|Default|GetFloatingPawnMovement) (* (* (Variables|Default|GetCurrentLaunchDirection) (* _launchcurve (Variables|Default|GetBaseLaunchVelocity))) (stale EventTick DeltaSeconds)) true)
      (bind _returnvalue_4 (Class|Pawn|ConsumeMovementInputVector))
      (Class|MovementComponent|MoveUpdatedComponent (Variables|Default|GetFloatingPawnMovement) _returnvalue_4 "0, 0, 0" true)
      (CallFunction|SpawnEmitter))
    (:Finished
      (CallFunction|DespawnEmitter))))

(event Custom|SpawnEmitter
  (bind _currentlaunchdirection (Variables|Default|GetCurrentLaunchDirection))
  (bind _cubetrails (Variables|Default|GetCubeTrails))
  (bind _returnvalue (* _currentlaunchdirection -1.0))
  ;[0.4319 1 0] ParticleStuff
  (Utilities|FlowControl|DoOnce false
    (:Completed
      (Utilities|IsValid _cubetrails
        (:Is%20Valid
          (Effects|Components|ParticleSystem|SetVectorParameter _cubetrails "EmitterDirection" (Math|Vector|MakeVector (.x _returnvalue) (.y _returnvalue) 0.6))
          (Components|Activation|Activate _cubetrails true))))))

(event Custom|DespawnEmitter
  (bind _currentlaunchdirection (Variables|Default|GetCurrentLaunchDirection))
  (bind _cubetrails (Variables|Default|GetCubeTrails))
  (bind _cubetrails_2 (Variables|Default|GetCubeTrails))
  (bind _returnvalue (* _currentlaunchdirection -1.0))
  ;[0.4319 1 0] ParticleStuff
  (Utilities|IsValid _cubetrails
    (:Is%20Valid
      (Components|Activation|Deactivate _cubetrails)
      (Utilities|FlowControl|DoOnce false) ; enters at Reset
    )
    (:Is%20Not%20Valid
      (Utilities|FlowControl|DoOnce false) ; enters at Reset
    )))

(event Custom|ControlEmitter
  (params (SpeedRate :type Float%20%28single-precision%29) (SpawnRate :type Float%20%28single-precision%29))
  (bind _cubetrails (Variables|Default|GetCubeTrails))
  ;[0.4319 1 0] ParticleStuff
  (Utilities|IsValid _cubetrails
    (:Is%20Valid
      (Effects|Components|ParticleSystem|SetFloatParameter _cubetrails "EmitterMin" (* SpeedRate (Variables|Default|GetBaseTrailSpeedMin)))
      (Effects|Components|ParticleSystem|SetFloatParameter _cubetrails "EmitterMax" (* SpeedRate (Variables|Default|GetBaseTrailSpeedMax)))
      (Effects|Components|ParticleSystem|SetFloatParameter _cubetrails "EmitterSpawnRate" (* (Variables|Default|GetBaseTrailSpawnRate) SpawnRate))
      (CallFunction|SetCubeIntensity SpawnRate))))

(event Custom|ShowBeam
  (params (BeamToLocation :type Vector))
  ;[1 1 1] BeamParticleStuff
  (if (> (Math|Vector|VectorLength (Class|Pawn|GetLastMovementInputVector)) 0.1)
    (Effects|Components|ParticleSystem|SetVectorParameter (Variables|Default|GetCubeBeam) "BeamEnd" BeamToLocation)
    (Utilities|FlowControl|DoOnce false :!label _label
      (:Completed
        (Components|Activation|Activate (Variables|Default|GetCubeBeam) false)
        (goto _label_2 Reset)))
    (else
      (Utilities|FlowControl|Sequence
        (:then_0
          (goto _label Reset))
        (:then_1
          (Utilities|FlowControl|DoOnce false :!label _label_2
            (:Completed
              (Components|Activation|Deactivate (Variables|Default|GetCubeBeam)))))))))

(event Custom|SetCubeIntensity
  (params (inIntensity :type Float%20%28single-precision%29))
  (bind _dynamiccubematerial (Variables|Default|GetDynamicCubeMaterial))
  ;[0.4319 1 0] ParticleStuff
  (Utilities|IsValid _dynamiccubematerial
    (:Is%20Valid
      (Rendering|Material|SetScalarParameterValue _dynamiccubematerial "Intensity" (* inIntensity (Variables|Default|GetBaseGlowIntensity)) :!class /Script/Engine.MaterialInstanceDynamic))))

(event EventTick
  (params (DeltaSeconds :type Float%20%28single-precision%29))
  ;[1 0 0.06404] CubeLaunch
)

(event EventBeginPlay
  (bind _returnvalue (Rendering|Material|CreateDynamicMaterialInstance (Variables|Default|GetCube) 0 "/Game/Materials/CubeMaterial.CubeMaterial" "None" :!class /Script/Engine.PrimitiveComponent))
  (Variables|Default|SetDynamicCubeMaterial _returnvalue))

(fn ConstructionScript)

(fn FindNearestDirection
  (params (X :type Float%20%28single-precision%29) (Y :type Float%20%28single-precision%29))
  (bind _output_get (LocalVariables|SettempX X))
  (bind _output_get_2 (LocalVariables|SettempY Y))
  (if (or (== (Math|Float|Round _output_get) 0) (== (Math|Float|Round _output_get_2) 0))
    (return (Math|Float|Round _output_get) (Math|Float|Round _output_get_2))
    (else
      (if (< (LocalVariables|GettempX) 0.0)
        (LocalVariables|SettempXlength (* (LocalVariables|GettempX) -1.0))
        (LocalVariables|SetxNegative true)
        (else
          (LocalVariables|SettempXlength (LocalVariables|GettempX))))
      (if (< (LocalVariables|GettempY) 0.0)
        (LocalVariables|SettempYlength (* (LocalVariables|GettempYlength) -1.0))
        (LocalVariables|SetyNegative true)
        (else
          (LocalVariables|SettempYlength (LocalVariables|GettempY))))
      (if (> (LocalVariables|GettempXlength) (LocalVariables|GettempYlength))
        (return (select (LocalVariables|GetxNegative) -1 1) 0)
        (else
          (return 0 (select (LocalVariables|GetyNegative) -1 1)))))))